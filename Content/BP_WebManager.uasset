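; BP_WebManager is an actor that builds a sagging web strand between a start and end position and holds node and edge data for a web.
; SetupSpline runs at construction and BeginPlay, adding one spline mesh over the first segment before rebuilding a three-point spline with its midpoint lowered by HangAmount.
; TryShootWeb, uncalled here, line-traces between the endpoints and on a hit records a node-to-node edge with its rest length.
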(event `self.ReceiveBeginPlay`
  (`self.SetupSpline`))

(fn `ConnectStrand`
  (bind _nodebindex (`self.NodeBIndex`))
  (bind _nodeaindex (`self.NodeAIndex`))
  (`KismetArrayLibrary.Array_Add` (`self.WebEdges`) (make `/Game/Assets/S_WebEdge` _nodeaindex _nodebindex (`KismetMathLibrary.Vector_Distance` (`.WorldPosition_11_FEE9D91D4F38D1D9415ED3BF149F18A4` (break `/Game/Assets/S_WebNode` (`|GetArrayItem` (`self.WebNodes`) _nodeaindex))) (`.WorldPosition_11_FEE9D91D4F38D1D9415ED3BF149F18A4` (break `/Game/Assets/S_WebNode` (`|GetArrayItem` (`self.WebNodes`) _nodebindex)))) null)))

(fn `CreateRopeMesh `
  (bind (_location _tangent) (`SplineComponent.GetLocationAndTangentAtSplinePoint` (`self.Spline`) 0 "Local"))
  (bind (_location_2 _tangent_2) (`SplineComponent.GetLocationAndTangentAtSplinePoint` (`self.Spline`) 1 "Local"))
  (bind _returnvalue (`AddComponent|NODE_AddSplineMeshComponent-0` :`RelativeTransform` (`KismetMathLibrary.MakeTransform` (0.0 0.0 0.0) (struct :`Yaw` 154.0) (2.0 3.0 54.0))))
  (bind _output_get (set `self.RopeMesh` _returnvalue))
  (`SplineMeshComponent.SetStartAndEnd` _output_get _location _tangent _location_2 _tangent_2 true))

(fn `SetupSpline`
  (bind (_returnvalue_x _returnvalue_y _returnvalue_z) (`KismetMathLibrary.BreakVector` (/ (+ (`self.StartPosition `) (`self.EndPosition `)) 2)))
  (`self.CreateRopeMesh `)
  (`SplineComponent.ClearSplinePoints` (`self.Spline`) true)
  (`SplineComponent.AddSplinePoint` (`self.Spline`) (`self.StartPosition `) "World" true)
  (`SplineComponent.AddSplinePoint` (`self.Spline`) (`KismetMathLibrary.MakeVector` _returnvalue_x _returnvalue_y (- _returnvalue_z (`self.HangAmount`))) "World" true)
  (`SplineComponent.AddSplinePoint` (`self.Spline`) (`self.EndPosition `) "World" true)
  (`KismetSystemLibrary.PrintString` "OLDU BİŞİLER"))

(fn `TryShootWeb `
  (bind (_outhit _returnvalue) (`KismetSystemLibrary.LineTraceSingle` (`self.StartPosition `) (`self.EndPosition `) "TraceTypeQuery1"))
  (if _returnvalue
    (`self.ConnectStrand`)))

(fn `UserConstructionScript`
  (`self.SetupSpline`))