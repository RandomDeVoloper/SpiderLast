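; BP_Sound is a Blueprint that plays the OIIA cue as a 2D sound in response to cat spins.
; When OnCatSpinned fires and BisPlaying is false, it sets Spinning and increments the SpinnedCats counter.
; Playback volume scales with that counter and the cue's own volume multiplier, plus a small offset, clamped to a fixed range.
; The graph never sets BisPlaying itself.
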(event `OnCatSpinned`
  (if (not (`self.bisPlaying`))
    (set `self.bSpinning` true)
    (bind _output_get (set `self.Audio` "/Game/Assets/Sounds/S_OIIA_Cue.S_OIIA_Cue"))
    (`/Engine/EditorBlueprintResources/StandardMacros.IncrementFloat` (`self.SpinnedCats`)
      (:`  `
        (`GameplayStatics.PlaySound2D` _output_get (`KismetMathLibrary.FClamp` (+ (* (`self.SpinnedCats`) (`SoundCue.VolumeMultiplier` _output_get)) 0.1) 0.1 1.5) 1.0 0.0 null null)))))