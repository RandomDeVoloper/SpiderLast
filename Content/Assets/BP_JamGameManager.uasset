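; Game manager Blueprint that tracks spun cats and triggers the win state for a game jam game.
; RegisterSpinnedCat increments a counter and, once it reaches the target count, sets a GameWon flag so the win fires only once.
; HandleGameWin then creates the WBP_Won widget and adds it to the viewport.
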(fn `HandleGameWin`
  (if (`self.bGameWon`)
    (bind _returnvalue (`|CreateWidget` "/Game/WBP_Won.WBP_Won_C"))
    (`UserWidget.AddToViewport` _returnvalue 0)))

(fn `RegisterSpinnedCat`
  (bind _output_get (set `self.SpinnedCats` (+ (`self.SpinnedCats`) 1)))
  (if (and (>= _output_get (`self.TargetCats`)) (not (`self.bGameWon`)))
    (set `self.bGameWon` true)
    (`self.HandleGameWin`)))

(fn `UserConstructionScript`)