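; Actor component for the Spider assets that tracks a single clamped stat with optional automatic drain.
; A looping half-second timer lowers the value by the drain rate while auto drain is on, firing OnStatDepleted once when it reaches zero.
; ModifyStat adds a clamped amount and fires OnStatRecovered when a depleted stat rises above zero.
; GetPercent returns the current-to-max ratio.
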(event `self.ReceiveBeginPlay`
  (`KismetSystemLibrary.K2_SetTimerDelegate` (delegate `DrainTick`) 0.5 true))

(event `DrainTick`
  (if (`self.bAutoDrain`)
    (bind _output_get (set `self.CurrentValue` (`KismetMathLibrary.FClamp` (- (`self.CurrentValue`) (* 0.5 (`self.DrainRate`))) 0.0 (`self.MaxValue`))))
    (if (and (<= _output_get 0.0) (not (`self.bDepletedFired`)))
      (set `self.bDepletedFired` true)
      (`self.OnStatDepleted`))))

(fn `GetPercent`
  (returns (Percent :type "Float (double-precision)"))
  (return (/ (`self.CurrentValue`) (`KismetMathLibrary.FMax` (`self.MaxValue`) 1.0))))

(fn `ModifyStat`
  (params (InceaseAmount :type "Float (double-precision)"))
  (bind _output_get (set `self.CurrentValue` (`KismetMathLibrary.FClamp` (+ InceaseAmount (`self.CurrentValue`)) 0.0 (`self.MaxValue`))))
  (if (> _output_get 0.0)
    (if (`self.bDepletedFired`)
      (set `self.bDepletedFired` false)
      (`self.OnStatRecovered`))))