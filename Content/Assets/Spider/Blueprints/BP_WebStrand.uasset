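; Spider web strand actor that spans two world points as a sagging, collidable thread.
; InitStrand rebuilds a three-point spline, raised by WebHeight, with the midpoint lowered in proportion to span length to fake tension.
; BuildStrandMesh then adds a thin cylinder spline mesh per segment, following the spline tangents.
; Each segment uses a custom collision object channel, blocks pawns and world static, and generates overlap events.
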(fn `BuildStrandMesh`
  (bind _strandspline (`self.StrandSpline`))
  (for _index (range (+ (- (`SplineComponent.GetNumberOfSplinePoints` (`self.StrandSpline`)) 2) 1))
    (bind _returnvalue (`AddComponent|NODE_AddSplineMeshComponent-0` :`bManualAttachment` true))
    (`SceneComponent.SetMobility` _returnvalue "Movable")
    (`SceneComponent.K2_AttachToComponent` _returnvalue (`self.StrandSpline`) "None" "KeepRelative" "KeepRelative" "KeepRelative" true)
    (`StaticMeshComponent.SetStaticMesh` _returnvalue "/Game/LevelPrototyping/Meshes/SM_Cylinder.SM_Cylinder")
    (bind _returnvalue_2 (+ _index 1))
    (`SplineMeshComponent.SetStartAndEnd` _returnvalue (`SplineComponent.GetLocationAtSplinePoint` _strandspline _index "Local") (`SplineComponent.GetTangentAtSplinePoint` _strandspline _index "Local") (`SplineComponent.GetLocationAtSplinePoint` _strandspline _returnvalue_2 "Local") (`SplineComponent.GetTangentAtSplinePoint` _strandspline _returnvalue_2 "Local") true)
    (`SplineMeshComponent.SetStartScale` _returnvalue (0.05 0.05) true)
    (`SplineMeshComponent.SetEndScale` _returnvalue (0.05 0.05) true)
    ; Ağın collisionu ayarlandı
    (`PrimitiveComponent.SetCollisionEnabled` _returnvalue "QueryAndPhysics")
    (`PrimitiveComponent.SetCollisionObjectType` _returnvalue "ECC_GameTraceChannel2")
    (`PrimitiveComponent.SetCollisionResponseToChannel` _returnvalue "ECC_WorldStatic" "ECR_Block")
    (`PrimitiveComponent.SetCollisionResponseToChannel` _returnvalue "ECC_Pawn" "ECR_Block")
    (set `PrimitiveComponent.bGenerateOverlapEvents` true _returnvalue)))

(fn `InitStrand`
  (params (`StartPoint ` :type "Vector Structure") (`EndPoint ` :type "Vector Structure"))
  (bind _returnvalue (+ `StartPoint ` (`KismetMathLibrary.MakeVector` 0.0 0.0 (`self.WebHeight`))))
  (bind _returnvalue_2 (+ `EndPoint ` (`KismetMathLibrary.MakeVector` 0.0 0.0 (`self.WebHeight`))))
  ; Comment
  (`SplineComponent.ClearSplinePoints` (`self.StrandSpline`) true)
  ;;[0 0.15 0.01913 0.5] Start Point
  (`SplineComponent.AddSplinePoint` (`self.StrandSpline`) _returnvalue "World" false)
  ;;[0.15 0.114 0 0.5] FinalMidPoint
  (bind _output_get (set `self.FinalMidPoint ` (- (`KismetMathLibrary.VLerp` _returnvalue _returnvalue_2 0.5) (`KismetMathLibrary.MakeVector` 0.0 0.0 (* (`KismetMathLibrary.Vector_Distance` _returnvalue _returnvalue_2) 0.06)))))
  (`SplineComponent.AddSplinePoint` (`self.StrandSpline`) _output_get "World" false)
  ;;[0.15 0.01324 0 0.5] END Point
  (`SplineComponent.AddSplinePoint` (`self.StrandSpline`) _returnvalue_2 "World" true)
  ;; Spline spawnlama
  (`self.BuildStrandMesh`))

(fn `UserConstructionScript`)