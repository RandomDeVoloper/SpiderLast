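; BP_SpinningCat is a cat actor that reacts when BP_Spider overlaps its Box component.
; The overlap tests the Spinning flag and, only when already true, sets it again, activates BPSound, calls its OnCatSpinned and prints debug text.
; The construction script turns off RotatingMovement auto-activation, and nothing here activates it.
; A disconnected DoOnce leading to the same check never runs.
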(event `self.Box.OnComponentBeginOverlap`
  (params (OverlappedComponent :type "PrimitiveComponent Object Reference") (OtherActor :type "Actor Object Reference") (OtherComp :type "PrimitiveComponent Object Reference") (OtherBodyIndex :type Integer) (bFromSweep :type Boolean) (SweepResult :type "HitResult Structure (by ref)"))
  (cast `/Game/Assets/Spider/Blueprints/Character/BP_Spider` OtherActor)
  (if (`self.bSpinning`)
    (set `self.bSpinning` true)
    (`ActorComponent.SetActive` (`self.BP_Sound`) true false)
    (`/Game/BP_Sound.OnCatSpinned` (`self.BP_Sound`))
    (`KismetSystemLibrary.PrintString` "asgdhagags")))

(fn `UserConstructionScript`
  (`ActorComponent.SetAutoActivate` (`self.RotatingMovement`) false))