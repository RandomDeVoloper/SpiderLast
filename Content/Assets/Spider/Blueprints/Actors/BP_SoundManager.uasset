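; BP_SoundManager is a sound manager in the Spider game that makes its audio louder as cats are spinned.
; Its construction script starts the Audio component playing from the beginning.
; Each OnCatSpinned event increments a counter, scales it by VolumeStep above a small base, clamps the result and applies it as the volume multiplier.
; The new multiplier is also printed to screen.
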(event `OnCatSpinned`
  (`/Engine/EditorBlueprintResources/StandardMacros.IncrementFloat` (`self.SpinnedCats`)
    (:`  `
      (bind _output_get (set `self.VolumeMultiplier` (`KismetMathLibrary.FClamp` (+ (* (`self.SpinnedCats`) (`self.VolumeStep`)) 0.1) 0.1 1.5)))
      (`AudioComponent.SetVolumeMultiplier` (`self.Audio`) _output_get)
      (`KismetSystemLibrary.PrintString` (`KismetStringLibrary.Conv_DoubleToString` _output_get) true true (struct :`R` 1.0 :`G` 0.69327 :`A` 1.0)))))

(fn `UserConstructionScript`
  (`AudioComponent.Play` (`self.Audio`) 0.0))