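; BP_JameGameManager is a game manager that tracks the win condition of spinning a target number of cats.
; RegisterSpinnedCat increments a counter and, once it reaches TargetCats, sets a one-time GameWon flag and calls HandleGameWin.
; HandleGameWin creates the WBP_GameWon widget for the first player controller, but its AddToViewport call is disconnected, so this Blueprint never displays it.
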(event `HandleGameWin`
  (bind _returnvalue (`|CreateWidget` "/Game/WBP_GameWon.WBP_GameWon_C" (`GameplayStatics.GetPlayerController` 0))))

(fn `RegisterSpinnedCat`
  (bind _output_get (set `self.SpinnedCats` (+ (`self.SpinnedCats`) 1)))
  (if (and (>= _output_get (`self.TargetCats`)) (not (`self.bGameWon`)))
    (set `self.bGameWon` true)
    (`self.HandleGameWin`)))

(fn `UserConstructionScript`)