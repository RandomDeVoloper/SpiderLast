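; BP_Sound is an actor that plays auto-activated audio whose volume rises as cats are spun, and it also tracks the win condition.
; The Add and Subtract keys adjust a clamped user volume, while OnCatSpinned derives a clamped game volume from the spun-cat count.
; ApplyVolume multiplies both onto the Audio component.
; Reaching the target cat count sets GameWon once, with only a debug print.
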(event `self.ReceiveBeginPlay`
  ; İNPUT AÇMA
  (bind _returnvalue (`GameplayStatics.GetActorOfClass` "/Game/Assets/Spider/Blueprints/Character/BP_Spider.BP_Spider_C"))
  (set `self.PlayerRef` _returnvalue)
  (`self.EnableInput` (`GameplayStatics.GetPlayerController` 0)))

(event `Key|Add`
  (params (Key :type "Key Structure"))
  (bind _returnvalue (+ (`self.UserVolume`) 0.2))
  ; VOLUME + -
  (:`Pressed`
    (`KismetSystemLibrary.PrintString` (`KismetStringLibrary.Conv_DoubleToString` _returnvalue))
    (set `self.UserVolume` (`KismetMathLibrary.FClamp` _returnvalue 0.5 3.0))
    (`self.ApplyVolume`)))

(event `Key|Subtract`
  (params (Key :type "Key Structure"))
  (bind _returnvalue (- (`self.UserVolume`) 0.2))
  ; VOLUME + -
  (:`Pressed`
    (`KismetSystemLibrary.PrintString` (`KismetStringLibrary.Conv_DoubleToString` _returnvalue))
    (set `self.UserVolume` (`KismetMathLibrary.FClamp` _returnvalue 0.5 3.0))
    (`self.ApplyVolume`)))

(event `OnCatSpinned`
  (bind _spinnedcats (`self.SpinnedCats`))
  (`KismetSystemLibrary.PrintString` "onspinned")
  (bind _result (`/Engine/EditorBlueprintResources/StandardMacros.IncrementInt` _spinnedcats)
    (:`  `
      (set `self.gameVol` (`KismetMathLibrary.FClamp` (+ (* _spinnedcats (`self.VolumeStep`)) 0.1) 0.5 4.0))
      (`self.ApplyVolume`)
      (if (and (>= _result (`self.TargetCats`)) (not (`self.bGameWon`)))
        (bind _output_get (set `self.bGameWon` true))
        (`KismetSystemLibrary.PrintString` (`KismetStringLibrary.Conv_BoolToString` _output_get))))))

(fn `ApplyVolume`
  (`KismetSystemLibrary.PrintString` "applyvolume")
  (`AudioComponent.SetVolumeMultiplier` (`self.Audio`) (* (`self.gameVol`) (`self.UserVolume`))))

(fn `UserConstructionScript`
  (`ActorComponent.SetAutoActivate` (`self.Audio`) true))