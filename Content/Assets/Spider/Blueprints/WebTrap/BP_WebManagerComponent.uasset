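; Web manager component for the spider's web trap that places web anchor points and links them with strands.
; TryShootWeb sphere-traces between start and end positions, storing each hit as a node with position, normal and component.
; Once two nodes exist, ConnectStrand spawns a BP_WebStrand between the pending-index node and its predecessor, recording an edge with rest length.
; A timed reset of the pending index and debug printing are left unconnected.
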(fn `ConnectStrand`
  (bind _nodebindex (`self.NodeBIndex`))
  (bind _nodeaindex (`self.NodeAIndex`))
  (bind _worldposition (break `/Game/Assets/S_WebNode` (`|GetArrayItem` (`self.WebNodes`) _nodebindex)))
  (bind _worldposition_2 (break `/Game/Assets/S_WebNode` (`|GetArrayItem` (`self.WebNodes`) _nodeaindex)))
  ;[0.008023 0.02956 0.07819] A and B index making strcty
  (bind _returnvalue (`|SpawnActorFromClass` "/Game/BP_WebStrand.BP_WebStrand_C" (`KismetMathLibrary.MakeTransform` _worldposition_2) "AlwaysSpawn" "MultiplyWithRoot" null null))
  (`/Game/BP_WebStrand.InitStrand` _returnvalue _worldposition_2 _worldposition)
  (`KismetArrayLibrary.Array_Add` (`self.WebEdges`) (make `/Game/Assets/S_WebEdge` _nodeaindex _nodebindex (`KismetMathLibrary.Vector_Distance` _worldposition_2 _worldposition) _returnvalue)))

(fn `TryShootWeb `
  (bind _returnvalue (`KismetArrayLibrary.Array_Length` (`self.WebNodes`)))
  (bind _returnvalue_2 (- _returnvalue 1))
  ;[0.15 0.1264 0] Trace
  ;; A ve b nin değer ayarlaması
  (bind _output_get (set `self.NodeAIndex` (`self.PendingNodeIndex `)))
  (set `self.NodeBIndex` (- _output_get 1))
  (bind (_outhit _returnvalue_3) (`KismetSystemLibrary.SphereTraceSingle` :`Start` (`self.StartPosition `) :`End` (`self.EndPosition `) :`Radius` 10.0 :`TraceChannel` "TraceTypeQuery1" :`DrawTime` 15.0))
  (if _returnvalue_3
    (bind (_bblockinghit _binitialoverlap _time _distance _location _impactpoint _normal _impactnormal _physmat _hitactor _hitcomponent) (`GameplayStatics.BreakHitResult` _outhit))
    (`KismetArrayLibrary.Array_Add` (`self.WebNodes`) (make `/Game/Assets/S_WebNode` _impactpoint _impactnormal _hitcomponent _returnvalue))
    (if (>= _returnvalue 2)
      ;[0 0.15 0.1192] Ağ 2 den fazlaysa pendingi 1 azaltma
      (`self.ConnectStrand`)
      (set `self.PendingNodeIndex ` _returnvalue_2)
      (else
        ;[0.15 0 0.09781 0] yeterli bağ oluşabilecek ağ var mı kontrolü sonradan belirli bir süre sonra sıfırlanır burası
        (bind _result (`/Engine/EditorBlueprintResources/StandardMacros.DecrementInt` _returnvalue_2)
          (:`  `
            (set `self.PendingNodeIndex ` _result)))))))